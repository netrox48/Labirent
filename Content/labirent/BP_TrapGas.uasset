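; BP_TrapGas is a gas trap in the labirent (maze) folder that applies damage over time to the player character standing inside it.
; DamageBox overlap starts and clears a looping DOT timer that passes DOTDamage to the character's HealthUpdate at each DOTTime interval.
; It binds to the character's DPTrap dispatcher on BeginPlay, and a matching TrapType disables the box's collision and destroys the Gas component.
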(event OnComponentBeginOverlap(DamageBox)
  (params (OverlappedComponent :type Primitive%20Component%20Object%20Reference) (OtherActor :type Actor%20Object%20Reference) (OtherComp :type Primitive%20Component%20Object%20Reference) (OtherBodyIndex :type Integer) (bFromSweep :type Boolean) (SweepResult :type Hit%20Result%20Structure%20%28by%20ref%29))
  (if (== OtherActor (Variables|Default|GetAs%20BP%20Character))
    (Utilities|Time|SetTimerbyFunctionName 0 "DOT" (Variables|Default|GetDOT_Time) true)))

(event OnComponentEndOverlap(DamageBox)
  (params (OverlappedComponent :type Primitive%20Component%20Object%20Reference) (OtherActor :type Actor%20Object%20Reference) (OtherComp :type Primitive%20Component%20Object%20Reference) (OtherBodyIndex :type Integer))
  (if (== OtherActor (Variables|Default|GetAs%20BP%20Character))
    (Utilities|Time|ClearTimerbyFunctionName 0 "DOT")))

(event Custom|DP_Trap_Event
  (params (Trap%20Type :type TrapType%20Enum :default "NewEnumerator0"))
  (if (Utilities|Enum|Equal(Enum) Trap%20Type (Variables|Default|GetTrapType))
    (Collision|SetCollisionEnabled (Variables|Default|GetDamageBox) "NoCollision")
    (Components|DestroyComponent (Variables|Default|Getgas))))

(event Custom|DOT
  (Default|HealthUpdate (Variables|Default|GetAs%20BP%20Character) (Variables|Default|GetDOT_Damage)))

(event EventBeginPlay
  (bind _asbp_character (Utilities|Casting|CastToBP_Character (Game|GetPlayerCharacter 0)))
  (bind _output_get (Variables|Default|SetAs%20BP%20Character _asbp_character))
  (EventDispatchers|BindEventtoDPTrap _output_get (delegate Custom|DP_Trap_Event)))

(fn ConstructionScript)