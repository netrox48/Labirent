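; BP_TrapSpike is a spike trap that hurts the player character.
; Entering its activation box plays a timeline that moves the spike mesh along Z, while overlapping a separate damage box reduces health.
; It binds to a trap event on BP_Character at BeginPlay.
; A matching TrapType permanently disarms it by lowering the spikes, disabling damage collision and destroying the timeline, which the validity check then blocks.
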(event OnComponentBeginOverlap(DamageBox)
  (params (OverlappedComponent :type Primitive%20Component%20Object%20Reference) (OtherActor :type Actor%20Object%20Reference) (OtherComp :type Primitive%20Component%20Object%20Reference) (OtherBodyIndex :type Integer) (bFromSweep :type Boolean) (SweepResult :type Hit%20Result%20Structure%20%28by%20ref%29))
  (if (== OtherActor (Variables|Default|GetAs%20BP%20Character))
    (Default|HealthUpdate (Variables|Default|GetAs%20BP%20Character) -3e+01)))

(event OnComponentBeginOverlap(ActivatitonBox)
  (params (OverlappedComponent :type Primitive%20Component%20Object%20Reference) (OtherActor :type Actor%20Object%20Reference) (OtherComp :type Primitive%20Component%20Object%20Reference) (OtherBodyIndex :type Integer) (bFromSweep :type Boolean) (SweepResult :type Hit%20Result%20Structure%20%28by%20ref%29))
  (if (== OtherActor (Variables|Default|GetAs%20BP%20Character))
    (Variables|Default|GetSpikes%20TL
      (:then
        (bind _newtrack_0 (Timeline|Spikes%20TL Play)
          (:Update
            (Transformation|SetRelativeLocation (Variables|Default|GetSM_Spikes) (Math|Vector|MakeVector 0.0 0.0 _newtrack_0) false false))))
      (:else))))

(event Custom|DP_Trap_Event
  (params (Trap%20Type :type TrapType%20Enum :default "NewEnumerator0"))
  (if (Utilities|Enum|Equal(Enum) Trap%20Type (Variables|Default|GetTrap%20Type))
    (Transformation|SetRelativeLocation (Variables|Default|GetSM_Spikes) "0.000000,0.000000,-165.000000" false false)
    (Collision|SetCollisionEnabled (Variables|Default|GetDamageBox) "NoCollision")
    (Components|DestroyComponent (Variables|Default|GetSpikes%20TL))))

(event EventBeginPlay
  (bind _asbp_character (Utilities|Casting|CastToBP_Character (Game|GetPlayerCharacter 0)))
  (bind _output_get (Variables|Default|SetAs%20BP%20Character _asbp_character))
  (EventDispatchers|BindEventtoDPTrap _output_get (delegate Custom|DP_Trap_Event)))

(fn ConstructionScript)