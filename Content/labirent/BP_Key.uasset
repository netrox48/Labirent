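; BP_Key is a key pickup actor that grants a numbered key to the player through the game mode.
; On BeginPlay it caches BP_MyGameMode, and on Interact it overwrites that game mode's Keys value with its KeyNumber.
; It then prints an acquired message using the key's name from Names and destroys itself.
; The construction script colors the sphere green or red based on KeyNumber.
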(event EventBeginPlay
  (bind _asbp_my_game_mode (Utilities|Casting|CastToBP_MyGameMode (Game|GetGameMode)))
  (Variables|Default|Setgamemode _asbp_my_game_mode))

(event EventInteract
  (bind _output_get (Variables|/Game/labirent/BP_MyGameMode.BP_MyGameMode_C|SetKeys (Variables|Default|Getgamemode) (Variables|Default|GetKeyNumber)))
  (Development|PrintString (Utilities|String|Append "Key" (Utilities|Array|Get(acopy) (Variables|Default|GetNames) _output_get) "Acquired"))
  (Actor|DestroyActor))

(fn ConstructionScript
  (bind _sphere (Variables|Default|GetSphere))
  (switch int (Variables|Default|GetKeyNumber)
    (:1
      (Rendering|Material|SetMaterial _sphere 0 "/Game/labirent/MI_Green.MI_Green"))
    (:2
      (Rendering|Material|SetMaterial _sphere 0 "/Game/labirent/MI_Red.MI_Red"))))