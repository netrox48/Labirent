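; BP_Switch is an interactable switch in the labyrinth (labirent) game that turns off traps of a given TrapType.
; On BeginPlay it caches the player's BP_Character and shows the TrapType enum name on its TextRender.
; On Interact it calls the DPTrap dispatcher on that character with its TrapType and prints a message, so it holds no direct trap references.
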(event EventBeginPlay
  (bind _asbp_character (Utilities|Casting|CastToBP_Character (Game|GetPlayerCharacter 0)))
  (Variables|Default|SetAs%20BP%20Character _asbp_character)
  (Rendering|Components|TextRender|SetText (Variables|Default|GetTextRender) (Utilities|Text|ToText(String) (Utilities|String|EnumtoString (Variables|Default|GetTrap%20Type)))))

(event EventInteract
  (Default|CallDPTrap (Variables|Default|GetAs%20BP%20Character) (Variables|Default|GetTrap%20Type))
  (Development|PrintString "Turn Off Trap"))

(fn ConstructionScript)