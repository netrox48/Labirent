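; BP_Gold is a maze gold pickup with a random value, shown on its text render.
; The construction script rolls the value and calls Creat Mesh at three thresholds, so richer piles get more randomly offset and scaled meshes.
; BeginPlay caches BP_MyGameMode and adds a Coin_widget to the viewport per pickup.
; Interact adds the value to the game mode's PlayerGold, prints the total and destroys the actor.
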(event EventInteract
  (bind _output_get (Variables|/Game/labirent/BP_MyGameMode.BP_MyGameMode_C|SetPlayerGold (Variables|Default|GetGM%20Maze) (+ (Variables|/Game/labirent/BP_MyGameMode.BP_MyGameMode_C|GetPlayerGold (Variables|Default|GetGM%20Maze)) (Variables|Default|GetItemGold))))
  (Development|PrintString (Utilities|String|Append "Current Gold" (Utilities|String|ToString(Integer) _output_get)))
  (Actor|DestroyActor))

(event EventBeginPlay
  (Utilities|FlowControl|Sequence
    (:then_0
      (bind _asbp_my_game_mode (Utilities|Casting|CastToBP_MyGameMode (Game|GetGameMode)))
      (Variables|Default|SetGM%20Maze _asbp_my_game_mode)
      (Rendering|Components|TextRender|SetText (Variables|Default|GetTextRender) (Utilities|Text|ToText(Integer) (Variables|Default|GetItemGold))))
    (:then_1
      (bind _returnvalue (UserInterface|CreateWidget "/Game/labirent/coin_widget.coin_widget_C"))
      (UserInterface|Viewport|AddtoViewport _returnvalue 0))))

(fn ConstructionScript
  (Variables|Default|SetItemGold (Math|Random|RandomIntegerinRange 1 99))
  (Utilities|CreatMesh (> (Variables|Default|GetItemGold) 76)
    (:Out
      _)
    (:False
      _))
  (Utilities|CreatMesh (> (Variables|Default|GetItemGold) 26)
    (:Out
      _)
    (:False
      _))
  (Utilities|CreatMesh (> (Variables|Default|GetItemGold) 1)))