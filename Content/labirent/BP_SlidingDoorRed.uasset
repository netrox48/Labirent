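; BP_SlidingDoorRed is a key-locked sliding door that opens on Interact when the game mode's Keys value equals its KeyNumber.
; A timeline lerps the door mesh's relative location from StartLoc to FinishLoc, with no closing logic; a mismatched key prints a message.
; The construction script sets the door's material to green or red from KeyNumber, so the color indicates the required key.
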(event EventInteract
  (bind _asbp_my_game_mode (Utilities|Casting|CastToBP_MyGameMode (Game|GetGameMode)))
  (if (== (Variables|/Game/labirent/BP_MyGameMode.BP_MyGameMode_C|GetKeys _asbp_my_game_mode) (Variables|Default|GetKeyNumber))
    (bind _newtrack_0 (Timeline|Door_Timeline Play)
      (:Update
        (Transformation|SetRelativeLocation (Variables|Default|GetSM_Door) (Math|Vector|Lerp(Vector) (Variables|Default|GetStartLoc) (Variables|Default|GetFinishLoc) _newtrack_0) false false)))
    (else
      (Development|PrintString "You dont have the correct key"))))

(fn ConstructionScript
  (bind _sm_door (Variables|Default|GetSM_Door))
  (switch int (Variables|Default|GetKeyNumber)
    (:1
      (Rendering|Material|SetMaterial _sm_door 0 "/Game/labirent/MI_Green.MI_Green"))
    (:2
      (Rendering|Material|SetMaterial _sm_door 0 "/Game/labirent/MI_Red.MI_Red"))))