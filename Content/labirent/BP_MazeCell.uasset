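; Configurable maze cell actor that builds one tile of the labyrinth, with optional walls, ceiling, light, trap and pickup.
; The construction script scales cube meshes from GridSize and WallHeight, and only sets trap child actors (spike, axe, gas, moving wall) on ceilinged cells with positive light intensity.
; BeginPlay spawns flagged medkit or gold and binds to the character's maze-gate event, which recolors a referenced SpotLight when IsInside is false.
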(event Custom|MazeGate_Event
  (params (IsInside? :type Boolean))
  (bind _spotlight (Variables|Default|GetSpotLight))
  (if (not IsInside?)
    (Utilities|IsValid _spotlight
      (:Is%20Valid
        (Rendering|Components|Light|SetLightColor (Variables|/Script/Engine.Light|GetLightComponent _spotlight) (Variables|Default|GetLightColor) true)))))

(event EventBeginPlay
  (Utilities|FlowControl|Sequence
    (:then_0
      (bind _asbp_character (Utilities|Casting|CastToBP_Character (Game|Player|GetPlayerPawn 0)))
      (Variables|Default|SetAs%20BP%20Character _asbp_character)
      (EventDispatchers|BindEventtoDPMazeGate _asbp_character (delegate Custom|MazeGate_Event)))
    (:then_1
      (if (Variables|Default|GetMadeKit)
        (Game|SpawnActorfromClass "/Game/labirent/BP_Medkit.BP_Medkit_C" (Math|Transform|MakeTransform (.location (Math|Transform|MakeTransform (+ (Transformation|GetActorLocation) "250.000000,250.000000,100.000000"))) "0, 0, 0" "1.000000,1.000000,1.000000") "Undefined" "MultiplyWithRoot" 0 0)))
    (:then_2
      (if (Variables|Default|GetGold)
        (Game|SpawnActorfromClass "/Game/labirent/BP_Gold.BP_Gold_C" (Math|Transform|MakeTransform (.location (Math|Transform|MakeTransform (+ (Transformation|GetActorLocation) "250.000000,250.000000,100.000000"))) "0, 0, 0" "1.000000,1.000000,1.000000") "Undefined" "MultiplyWithRoot" 0 0)))))

(fn ConstructionScript
  (bind _wallactor (Variables|Default|GetWallActor))
  (bind _childactor (Variables|Default|GetChildActor))
  (bind _gridsize (Variables|Default|GetGridSize))
  (LocalVariables|SetWallLenght _gridsize)
  (LocalVariables|SetWallThickness (* _gridsize 0.1))
  (Transformation|SetRelativeScale3D (Variables|Default|GetFloor) (Utilities|SizetoCubeScale (Math|Vector|MakeVector (LocalVariables|GetWallLenght) (LocalVariables|GetWallLenght) (LocalVariables|GetWallThickness))))
  (if (Variables|Default|GetWestWall)
    (AddComponent|AddStaticMeshComponent false (Math|Transform|MakeTransform (Math|Vector|MakeVector 0.0 0.0 0.0) "0, 0, 0" (Utilities|SizetoCubeScale (Math|Vector|MakeVector (LocalVariables|GetWallLenght) (LocalVariables|GetWallThickness) (Variables|Default|GetWallHeight))))))
  (if (Variables|Default|GetSouthWall)
    (AddComponent|AddStaticMeshComponent false (Math|Transform|MakeTransform (Math|Vector|MakeVector 0.0 0.0 0.0) "0, 0, 0" (Utilities|SizetoCubeScale (Math|Vector|MakeVector (LocalVariables|GetWallThickness) (LocalVariables|GetWallLenght) (Variables|Default|GetWallHeight))))))
  (if (Variables|Default|GetNorthWall)
    (AddComponent|AddStaticMeshComponent false (Math|Transform|MakeTransform (Math|Vector|MakeVector (- (LocalVariables|GetWallLenght) (LocalVariables|GetWallThickness)) 0.0 0.0) "0, 0, 0" (Utilities|SizetoCubeScale (Math|Vector|MakeVector (LocalVariables|GetWallThickness) (LocalVariables|GetWallLenght) (Variables|Default|GetWallHeight))))))
  (if (Variables|Default|GetEastWall)
    (AddComponent|AddStaticMeshComponent false (Math|Transform|MakeTransform (Math|Vector|MakeVector 0.0 (- (LocalVariables|GetWallLenght) (LocalVariables|GetWallThickness)) 0.0) "0, 0, 0" (Utilities|SizetoCubeScale (Math|Vector|MakeVector (LocalVariables|GetWallLenght) (LocalVariables|GetWallThickness) (Variables|Default|GetWallHeight))))))
  (if (Variables|Default|GetCeiling)
    (AddComponent|AddStaticMeshComponent false (Math|Transform|MakeTransform (Math|Vector|MakeVector 0.0 0.0 (Variables|Default|GetWallHeight)) "0, 0, 0" (Utilities|SizetoCubeScale (Math|Vector|MakeVector (LocalVariables|GetWallLenght) (LocalVariables|GetWallLenght) (LocalVariables|GetWallThickness)))))
    (if (> (Variables|Default|GetLightIntensity) 0.0)
      (bind _returnvalue (AddComponent|AddSpotLightComponent false (Math|Transform|MakeTransform (Math|Vector|MakeVector (* (LocalVariables|GetWallLenght) 0.5) (* (LocalVariables|GetWallLenght) 0.5) (* (Variables|Default|GetWallHeight) 0.9)) "-90.000000,0.000000,0.000000" "1.000000,1.000000,1.000000")))
      (Rendering|Components|Light|SetLightColor _returnvalue (Variables|Default|GetLightColor) true)
      (Rendering|Components|Light|SetIntensity _returnvalue (Variables|Default|GetLightIntensity))
      (switch Utilities|FlowControl|Switch|SwitchonTrapType (Variables|Default|GetTrapType)
        (:NewEnumerator0
          (Variables|Default|SetTrap false))
        (:NewEnumerator1
          (Variables|Default|SetTrap true)
          (ChildActorComponent|SetChildActorClass (Variables|Default|GetChildActor) "/Game/labirent/BP_TrapSpike.BP_TrapSpike_C"))
        (:NewEnumerator2
          (Variables|Default|SetTrap true)
          (ChildActorComponent|SetChildActorClass _childactor "/Game/labirent/Axe.Axe_C")
          (Transformation|SetWorldRotation _childactor (Variables|Default|GetTrap%20Rotation) false false))
        (:NewEnumerator3
          (Variables|Default|SetTrap true)
          (ChildActorComponent|SetChildActorClass (Variables|Default|GetChildActor) "/Game/labirent/BP_TrapGas.BP_TrapGas_C"))
        (:NewEnumerator4
          (Variables|Default|SetTrap true)
          (ChildActorComponent|SetChildActorClass _wallactor "/Game/labirent/WallMovement.WallMovement_C")
          (Transformation|SetWorldRotation _wallactor (Variables|Default|GetTrap%20Rotation) false false))))))