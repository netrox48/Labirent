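; Game mode for a maze game that adds the HUD widget at BeginPlay and enforces a 90-second time limit.
; Tick checks game time, and once the limit passes it finds every BP_MazeCell and turns its spotlight red.
; This repeats every frame after timeout, printing a failure message once per cell, with no latch or game-end handling.
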(event EventBeginPlay
  (bind _returnvalue (UserInterface|CreateWidget "/Game/labirent/WBP_Hud.WBP_Hud_C" (Game|GetPlayerController 0)))
  (bind _output_get (Variables|Default|SetHud _returnvalue))
  (UserInterface|Viewport|AddtoViewport _output_get 0))

(event EventTick
  (params (DeltaSeconds :type Float%20%28single-precision%29))
  (if (> (Utilities|Time|GetGameTimeinSeconds) 9e+01)
    (bind _outactors (Actor|GetAllActorsOfClass "/Game/labirent/BP_MazeCell.BP_MazeCell_C"))
    (for _array_element _outactors
      (Rendering|Components|Light|SetLightColor (Actor|GetComponentbyClass _array_element "/Script/Engine.SpotLightComponent") "(R=1.000000,G=0.000000,B=0.000000,A=1.000000)" true)
      (Development|PrintString "You have failed!"))))

(fn ConstructionScript)